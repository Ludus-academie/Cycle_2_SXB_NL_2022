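; Archived player pawn that moves and looks via input axes and grabs physics objects with a Physics Handle.
; Pressing Grab runs a debug-drawn visibility trace and grabs the hit component without checking for a hit; releasing lets go.
; The trace ends at controller forward times Distance, with no start offset added.
; Tick holds the handle target in front of the pawn along control rotation and prints debug text.
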(event `InputAction|Grab`
  (params (Key :type "Key Structure"))
  (bind _physicshandle (`self.PhysicsHandle`))
  ;[1 1 1] Grab Actor (Physics Actor)
  (:`Pressed`
    (bind _outhit (`KismetSystemLibrary.LineTraceSingle` :`Start` (`self.K2_GetActorLocation`) :`End` (* (`self.GetActorForwardVector` (`GameplayStatics.GetPlayerController` 0)) (`self.Distance`)) :`TraceChannel` "TraceTypeQuery1" :`DrawDebugType` "Persistent"))
    (if true
      (bind (_bblockinghit _binitialoverlap _time _distance _location _impactpoint _normal _impactnormal _physmat _hitactor _hitcomponent) (`GameplayStatics.BreakHitResult` _outhit))
      (`PhysicsHandleComponent.GrabComponentAtLocation` _physicshandle _hitcomponent "None" _location)
      (`KismetSystemLibrary.PrintString` (`KismetSystemLibrary.GetDisplayName` (`PhysicsHandleComponent.GetGrabbedComponent` _physicshandle)))))
  (:`Released`
    (`PhysicsHandleComponent.ReleaseComponent` (`self.PhysicsHandle`))))

(event `InputAxis|Forward/Backward`
  (params (AxisValue :type "Float (single-precision)"))
  ;[1 1 1] Movement
  (`self.AddMovementInput` (`self.GetActorForwardVector` (`GameplayStatics.GetPlayerController` 0)) AxisValue))

(event `InputAxis|Left/Right`
  (params (AxisValue :type "Float (single-precision)"))
  ;[1 1 1] Movement
  (`self.AddMovementInput` (`self.GetActorRightVector` (`GameplayStatics.GetPlayerController` 0)) AxisValue))

(event `self.ReceiveTick`
  (params (DeltaSeconds :type "Float (single-precision)"))
  ;[1 1 1] Set Handle Location and rotation
  (`PhysicsHandleComponent.SetTargetLocationAndRotation` (`self.PhysicsHandle`) (+ (`self.K2_GetActorLocation`) (* (`KismetMathLibrary.GetForwardVector` (`self.GetControlRotation`)) (`self.GrabLocation`))) (`self.GetControlRotation`))
  (`KismetSystemLibrary.PrintString` (`KismetSystemLibrary.GetDisplayName` null)))

(event `InputAxis|Turn`
  (params (AxisValue :type "Float (single-precision)"))
  ;[1 1 1] Movement
  (`self.AddControllerYawInput` AxisValue))

(event `InputAxis|LookUp`
  (params (AxisValue :type "Float (single-precision)"))
  ;[1 1 1] Movement
  (`self.AddControllerPitchInput` AxisValue))

(fn `UserConstructionScript`)